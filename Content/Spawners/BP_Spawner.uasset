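; BP_Spawner is an actor that spawns an actor at its root component's world location after a delay.
; BeginPlay enters a DoN gate limited by NumberToSpawn, waits SpawnDelay, increments SpawnedCount and calls SpawnCritter.
; Nothing loops back into the gate, so each BeginPlay yields a single spawn.
; SpawnCritter adjusts for collisions where possible but always spawns.
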(event `self.ReceiveBeginPlay`
  (`/Engine/EditorBlueprintResources/StandardMacros.Do N` (`self.NumberToSpawn`)
    (:`Exit`
      (`KismetSystemLibrary.Delay` (`self.SpawnDelay`))
      (bind _output_get (set `self.SpawnedCount` (+ (stale _output_get) 1)))
      (`self.SpawnCritter`))))

(fn `SpawnCritter`
  (locals (NewLocalVar_0 :type "Transform Structure"))
  (`|SpawnActorFromClass` "/Script/Engine.Actor" (`KismetMathLibrary.Conv_VectorToTransform` (`SceneComponent.K2_GetComponentLocation` (`self.DefaultSceneRoot`))) "AdjustIfPossibleButAlwaysSpawn" "OverrideRootScale" null null))

(fn `UserConstructionScript`)